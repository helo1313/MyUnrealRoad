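; BP_Car is a traffic car actor that hands itself to its WBP_CarInfo widget on BeginPlay.
; Tick only calls the parent implementation.
; A disconnected Blueprint car-following path traces ahead, then accelerates when clear or adjusts speed to the car in front, targeting half that car's speed inside the safe distance.
; MoveActorBP, which moves the actor forward by its speed, is not called in this graph.
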(event EventTick
  (params (DeltaSeconds :type Float%20%28single-precision%29))
  (|CallParentFunction DeltaSeconds))

(event EventBeginPlay
  (bind _aswbp_car_info (Utilities|Casting|CastToWBP_CarInfo (UserInterface|GetWidget (Variables|Default|GetWidget))))
  (Variables|/Game/MyUnrealRoad/Core/Car/WBP_CarInfo.WBP_CarInfo_C|SetCarRef _aswbp_car_info self))

(fn ConstructionScript)

(fn MoveActorBP
  (params (B :type Float%20%28single-precision%29))
  (Transformation|SetActorLocation (+ (Transformation|GetActorLocation) (* (Math|Vector|GetForwardVector (Transformation|GetActorRotation)) (* (Variables|Default|GetSpeedBP) B))) false false))

(fn AccelerateBP
  (params (Delta :type Float%20%28single-precision%29))
  (Variables|Default|SetSpeedBP (Math|Float|Clamp(Float) (+ (Variables|Default|GetSpeedBP) (* Delta 1.2e+02)) 0.0 (Variables|Default|GetMaxSpeedBP))))

(fn DecelerateBP
  (params (HitedActor :type Actor%20Object%20Reference) (Distance :type Float%20%28single-precision%29) (Delta :type Float%20%28single-precision%29))
  (bind _asbp_car (Utilities|Casting|CastToBP_Car HitedActor))
  (if (> (Variables|Default|GetSpeedBP) (Math|Float|SelectFloat (* (Variables|BP_Car_C|GetSpeedBP _asbp_car) 0.5) (Variables|BP_Car_C|GetSpeedBP _asbp_car) (< Distance (Variables|Default|GetSafeDistanceBP))))
    (Variables|Default|SetSpeedBP (Math|Float|Clamp(Float) (- (Variables|Default|GetSpeedBP) (* Delta 1.2e+02)) 0.0 (Variables|Default|GetMaxSpeedBP)))
    (else
      (CallFunction|AccelerateBP Delta))))